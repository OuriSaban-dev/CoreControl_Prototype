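; BP_TargetDummy is a damageable target that slides side to side along world Y and respawns after being destroyed.
; Tick moves it, reversing direction whenever it is beyond MoveDistance from StartLocation, which is recorded at BeginPlay.
; At zero health it hides, disables collision, waits briefly, then restores itself at a random TargetSpawn-tagged actor.
; StartLocation resets from a separate random pick, so it can differ from the spawn point.
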(event `self.ReceiveTick`
  (params (DeltaSeconds :type "Float (single-precision)"))
  ; MOVEMENT - Side to Side
  (`self.K2_AddActorWorldOffset` (`KismetMathLibrary.MakeVector` 0.0 (* (* (`self.MoveSpeed`) (`self.MoveDirection`)) DeltaSeconds)))
  (if (> (`KismetMathLibrary.Vector_Distance` (`self.K2_GetActorLocation`) (`self.StartLocation`)) (`self.MoveDistance`))
    (set `self.MoveDirection` (* (`self.MoveDirection`) -1.0))))

(event `self.ReceiveAnyDamage`
  (params (Damage :type "Float (single-precision)") (DamageType :type "DamageType Object Reference") (InstigatedBy :type "Controller Object Reference") (DamageCauser :type "Actor Object Reference"))
  ; HEALTH - Take Damage
  (set `self.Health` (- (`self.Health`) Damage))
  (if (<= (`self.Health`) 0.0)
    ; RESPAWN - Hide and Reset
    (`self.SetActorHiddenInGame` true)
    (`self.SetActorEnableCollision` false)
    (`KismetSystemLibrary.Delay` 2.0)
    ; RESPAWN - Random Spawn
    (bind _outactors (`GameplayStatics.GetAllActorsWithTag` "TargetSpawn"))
    (bind _returnvalue (`self.K2_GetActorLocation` (`KismetArrayLibrary.Array_Random` _outactors)))
    (`self.K2_SetActorLocation` _returnvalue)
    (set `self.StartLocation` _returnvalue)
    (set `self.Health` 100.0)
    (`self.SetActorHiddenInGame` false)
    ;; Comment
    (`self.SetActorEnableCollision` true)))

(event `self.ReceiveBeginPlay`
  ; INIT - Start Position
  (set `self.StartLocation` (`self.K2_GetActorLocation`)))

(fn `UserConstructionScript`)