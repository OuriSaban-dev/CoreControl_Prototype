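; Capture zone actor that the player holds to win the round, reporting progress and neutral, contested or captured state to the HUD through BP_CoreControlGameMode.
; Trigger overlaps track the player and register living BP_BasicBots as contesters.
; Each tick prunes dead, hidden, invalid or fallen bots, then advances progress only while the player is inside uncontested, also feeding player control and crowd energy.
; Full progress locks the zone and ends the round in victory.
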(event `CompleteZoneCapture`
  (set `self.ZoneCaptured` true)
  (`/Game/Blueprints/Gameplay/BP_CoreControlGameMode.HUD_SetZoneCaptured` (`self.GameModeRef`))
  (`/Game/Blueprints/Gameplay/BP_CoreControlGameMode.EndRoundVictory` (`self.GameModeRef`)))

(event `CaptureZone`
  (params (DeltaSeconds :type "Float (double-precision)"))
  (bind _output_get (set `self.CaptureProgress` (`KismetMathLibrary.FClamp` (+ (* (`self.CaptureSpeed`) DeltaSeconds) (`self.CaptureProgress`)) 0.0 100.0)))
  (`/Game/Blueprints/Gameplay/BP_CoreControlGameMode.HUD_UpdateZoneProgress` (`self.GameModeRef`) _output_get)
  (`/Game/Blueprints/Gameplay/BP_CoreControlGameMode.AddPlayerControl` (`self.GameModeRef`) (* (`self.CaptureSpeed`) DeltaSeconds))
  (`/Game/Blueprints/Gameplay/BP_CoreControlGameMode.AddCrowdEnergy` (`self.GameModeRef`) (* (`self.CrowdGainRate`) DeltaSeconds))
  (if (>= (`self.CaptureProgress`) 100.0)
    (`self.CompleteZoneCapture`)))

(event `self.ReceiveBeginPlay`
  (bind _asbp_core_control_game_mode (cast `/Game/Blueprints/Gameplay/BP_CoreControlGameMode` (`GameplayStatics.GetGameMode`)))
  (set `self.GameModeRef` _asbp_core_control_game_mode))

(event `ProcessZoneState`
  (params (DelatSeconds :type "Float (double-precision)"))
  (if (`self.ZoneCaptured`)
    _
    (elif (`self.PlayerInZone`)
      (if (> (`KismetArrayLibrary.Array_Length` (`self.ContestingBots`)) 0)
        (`/Game/Blueprints/Gameplay/BP_CoreControlGameMode.HUD_SetZoneContested` (`self.GameModeRef`))
        (else
          (`self.CaptureZone` DelatSeconds)))
      (else
        (`/Game/Blueprints/Gameplay/BP_CoreControlGameMode.HUD_SetZoneNeutral` (`self.GameModeRef`))))))

(event `CleanContestList`
  (`KismetArrayLibrary.Array_Clear` (`self.ValidContestingBots`))
  (for _array_element (`self.ContestingBots`)
    (`/Engine/EditorBlueprintResources/StandardMacros.IsValid` _array_element
      (:`Is Valid`
        (if (and (and (not (`/Game/Blueprints/Gameplay/BP_BasicBot.IsDead` _array_element)) (not (`Actor.bHidden` _array_element))) (> (.z (`self.K2_GetActorLocation` _array_element)) -1000.0))
          (`KismetArrayLibrary.Array_Add` (`self.ValidContestingBots`) _array_element)))))
  (set `self.ContestingBots` (`self.ValidContestingBots`)))

(event `UnregisterBotContest`
  (params (Bot :type "/Game/Blueprints/Gameplay/BP_BasicBot Object Reference"))
  (`/Engine/EditorBlueprintResources/StandardMacros.IsValid` Bot
    (:`Is Valid`
      (if (`KismetArrayLibrary.Array_Contains` (`self.ContestingBots`) Bot)
        (`KismetArrayLibrary.Array_RemoveItem` (`self.ContestingBots`) Bot)))))

(event `RegisterBotContest`
  (params (Bot :type "/Game/Blueprints/Gameplay/BP_BasicBot Object Reference"))
  (`/Engine/EditorBlueprintResources/StandardMacros.IsValid` Bot
    (:`Is Valid`
      (if (not (`/Game/Blueprints/Gameplay/BP_BasicBot.IsDead` Bot))
        (if (not (`KismetArrayLibrary.Array_Contains` (`self.ContestingBots`) Bot))
          (`KismetArrayLibrary.Array_Add` (`self.ContestingBots`) Bot))))))

(event `ForceRemovePlayer`
  (set `self.PlayerInZone` false)
  (`/Game/Blueprints/Gameplay/BP_CoreControlGameMode.HUD_SetZoneNeutral` (`self.GameModeRef`)))

(event `self.ReceiveTick`
  (params (DeltaSeconds :type "Float (single-precision)"))
  (`self.CleanContestList`)
  (`self.ProcessZoneState` DeltaSeconds))

(event `self.ZoneTrigger.OnComponentBeginOverlap`
  (params (OverlappedComponent :type "PrimitiveComponent Object Reference") (OtherActor :type "Actor Object Reference") (OtherComp :type "PrimitiveComponent Object Reference") (OtherBodyIndex :type Integer) (bFromSweep :type Boolean) (SweepResult :type "HitResult Structure (by ref)"))
  (cast `/Game/ThirdPerson/Blueprints/BP_ThirdPersonCharacter` OtherActor
    (:`then`
      (set `self.PlayerInZone` true))
    (:`CastFailed`
      (bind _asbp_basic_bot (cast `/Game/Blueprints/Gameplay/BP_BasicBot` OtherActor))
      (`self.RegisterBotContest` _asbp_basic_bot))))

(event `self.ZoneTrigger.OnComponentEndOverlap`
  (params (OverlappedComponent :type "PrimitiveComponent Object Reference") (OtherActor :type "Actor Object Reference") (OtherComp :type "PrimitiveComponent Object Reference") (OtherBodyIndex :type Integer))
  (cast `/Game/ThirdPerson/Blueprints/BP_ThirdPersonCharacter` OtherActor
    (:`then`
      (set `self.PlayerInZone` false))
    (:`CastFailed`
      (bind _asbp_basic_bot (cast `/Game/Blueprints/Gameplay/BP_BasicBot` OtherActor))
      (`self.UnregisterBotContest` _asbp_basic_bot))))

(fn `UserConstructionScript`)