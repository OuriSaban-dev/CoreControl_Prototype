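; BP_BotSpawner populates the level with bots when play begins.
; On BeginPlay it gathers all actors carrying SpawnTag, then spawns BotCount instances of BotClass at unit scale.
; Each spawn takes location and rotation from random picks among those tagged actors, with no check against reusing a point.
; Spawning always succeeds regardless of collision, so bots can overlap.
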(event `self.ReceiveBeginPlay`
  (bind _outactors (`GameplayStatics.GetAllActorsWithTag` (`self.SpawnTag`)))
  (for _ (range (`self.BotCount`))
    (bind _outitem (`KismetArrayLibrary.Array_Random` _outactors))
    (`|SpawnActorFromClass` (`self.BotClass`) (`KismetMathLibrary.MakeTransform` (`self.K2_GetActorLocation` _outitem) (`self.K2_GetActorRotation` _outitem)) "AlwaysSpawn" "MultiplyWithRoot" null null)))

(fn `UserConstructionScript`)