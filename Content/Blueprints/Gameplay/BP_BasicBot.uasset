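; BP_BasicBot is an enemy bot that advances on the control zone while the round is active, moving faster as player score rises.
; Overlapping the player deals cooldown-limited contact damage, and a material swap signals when the player is within danger range.
; Damage applies swept knockback along its backward vector.
; At zero health it awards score, hides, then reuses itself at a random TargetSpawn actor with sound and marker effects.
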(event `self.ReceiveActorBeginOverlap`
  (params (OtherActor :type "Actor Object Reference"))
  (cast `/Game/ThirdPerson/Blueprints/BP_ThirdPersonCharacter` OtherActor)
  (bind _asbp_core_control_game_mode (cast `/Game/Blueprints/Gameplay/BP_CoreControlGameMode` (`GameplayStatics.GetGameMode`)))
  (if (`/Game/Blueprints/Gameplay/BP_CoreControlGameMode.RoundActive` _asbp_core_control_game_mode)
    (if (`self.CanDealDamage`)
      (set `self.CanDealDamage` false)
      (`GameplayStatics.ApplyDamage` OtherActor (`self.ContactDamage`))
      (`KismetSystemLibrary.Delay` (`self.DamageCooldown`))
      (set `self.CanDealDamage` true))))

(event `self.ReceiveTick`
  (params (DeltaSeconds :type "Float (single-precision)"))
  ; MOVEMENT - Side to Side
  (bind _asbp_core_control_game_mode (cast `/Game/Blueprints/Gameplay/BP_CoreControlGameMode` (`GameplayStatics.GetGameMode`)))
  (if (`/Game/Blueprints/Gameplay/BP_CoreControlGameMode.RoundActive` _asbp_core_control_game_mode)
    (`|ExecutionSequence`
      (:`then_0`
        (bind _asbp_third_person_character (cast `/Game/ThirdPerson/Blueprints/BP_ThirdPersonCharacter` (`GameplayStatics.GetPlayerCharacter` 0)))
        (set `self.BotMoveSpeed` (+ (* (`KismetMathLibrary.Conv_IntToDouble` (`/Game/ThirdPerson/Blueprints/BP_ThirdPersonCharacter.Score` _asbp_third_person_character)) 0.2) (`self.BaseBotMoveSpeed`)))
        (bind _outactors (`GameplayStatics.GetAllActorsOfClass` "/Game/Blueprints/Gameplay/BP_ControlZone.BP_ControlZone_C"))
        (bind _returnvalue (`self.K2_GetActorLocation` (`|GetArrayItem` _outactors)))
        (if (> (`KismetMathLibrary.Vector_Distance` _returnvalue (`self.K2_GetActorLocation`)) (`self.StopDistanceToZone`))
          (`self.K2_AddActorWorldOffset` (* (* (`KismetMathLibrary.GetForwardVector` (`KismetMathLibrary.FindLookAtRotation` (`self.K2_GetActorLocation`) _returnvalue)) (`self.BotMoveSpeed`)) DeltaSeconds) true)))
      (:`then_1`
        (if (<= (`KismetMathLibrary.Vector_Distance` (`self.K2_GetActorLocation`) (`self.K2_GetActorLocation` (`GameplayStatics.GetPlayerCharacter` 0))) (`self.DangerDistance`))
          (`PrimitiveComponent.SetMaterial` (`self.Cube`) 0 "/Game/LevelPrototyping/Materials/M_Bot_Danger.M_Bot_Danger")
          (else
            (`PrimitiveComponent.SetMaterial` (`self.Cube`) 0 "/Game/LevelPrototyping/Materials/M_Bot_Normal.M_Bot_Normal")))))))

(event `self.ReceiveAnyDamage`
  (params (Damage :type "Float (single-precision)") (DamageType :type "DamageType Object Reference") (InstigatedBy :type "Controller Object Reference") (DamageCauser :type "Actor Object Reference"))
  ; HEALTH - Take Damage
  (set `self.Health` (- (`self.Health`) Damage))
  (`self.K2_AddActorWorldOffset` (* (`self.GetActorForwardVector`) (* (`self.KnockbackStrength`) -1.0)) true)
  (if (<= (`self.Health`) 0.0)
    (bind _asbp_third_person_character (cast `/Game/ThirdPerson/Blueprints/BP_ThirdPersonCharacter` (`GameplayStatics.GetPlayerCharacter` 0)))
    (`/Game/ThirdPerson/Blueprints/BP_ThirdPersonCharacter.AddScore` _asbp_third_person_character 100)
    (`GameplayStatics.PlaySound2D` "/Game/sound/bot_death.bot_death" 1.0 1.0 0.0 null null)
    (`|SpawnActorFromClass` "/Game/Blueprints/BP_ImpactMarker.BP_ImpactMarker_C" (`KismetMathLibrary.MakeTransform` (`self.K2_GetActorLocation`) (struct) (2.0 2.0 2.0)) "AlwaysSpawn" "MultiplyWithRoot" null null)
    ; RESPAWN - Hide and Reset
    (`self.SetActorHiddenInGame` true)
    (`self.SetActorEnableCollision` false)
    (`KismetSystemLibrary.Delay` 2.0)
    ; RESPAWN - Random Spawn
    (bind _outactors (`GameplayStatics.GetAllActorsWithTag` "TargetSpawn"))
    (`self.K2_SetActorLocation` (`self.K2_GetActorLocation` (`KismetArrayLibrary.Array_Random` _outactors)))
    (set `self.Health` 100.0)
    (`GameplayStatics.PlaySound2D` "/Game/sound/bot_spawn.bot_spawn" 1.0 1.0 0.0 null null)
    (`|SpawnActorFromClass` "/Game/Blueprints/BP_ImpactMarker.BP_ImpactMarker_C" (`KismetMathLibrary.MakeTransform` (`self.K2_GetActorLocation`) (struct) (1.5 1.5 1.5)) "Undefined" "MultiplyWithRoot" null null)
    (`self.SetActorHiddenInGame` false)
    (`self.SetActorEnableCollision` true)))

(fn `UserConstructionScript`)