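; Game mode for a timed zone-control round where player and enemy control percentages compete, ending in victory, defeat or draw.
; Tick counts down the timer; a side reaching full control wins early, otherwise higher control wins at timeout.
; Full crowd energy triggers a temporary Overload state that resets energy afterwards.
; It also creates and relays updates to HUD and crosshair widgets, and records playtest telemetry printed at round end.
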(event `StartOverload`
  (set `self.OverloadActive` true)
  (`self.HUD_SetOverloadState`)
  (`KismetSystemLibrary.Delay` 20.0)
  (set `self.OverloadActive` false)
  (bind _output_get (set `self.CrowdEnergy` 0.0))
  (`self.HUD_UpdateCrowdEnergy` _output_get))

(event `HUD_SetZoneNeutral`
  (`/Engine/EditorBlueprintResources/StandardMacros.IsValid` (`self.HUDWidgetRef`)
    (:`Is Valid`
      (`/Game/Blueprints/WBP_HUD.SetZoneNeutral` (`self.HUDWidgetRef`)))))

(event `AddCrowdEnergy`
  (params (Amount :type "Float (double-precision)"))
  (if (and (`self.RoundActive`) (not (`self.MatchEnded`)))
    (set `self.CrowdEnergy` (`KismetMathLibrary.FClamp` (+ (`self.CrowdEnergy`) Amount) 0.0 100.0))
    (`self.HUD_UpdateCrowdEnergy` (`self.CrowdEnergy`))
    (if (and (>= (`self.CrowdEnergy`) 100.0) (not (`self.OverloadActive`)))
      (`self.StartOverload`))))

(event `HUD_SetZoneContested`
  (`/Engine/EditorBlueprintResources/StandardMacros.IsValid` (`self.HUDWidgetRef`)
    (:`Is Valid`
      (`/Game/Blueprints/WBP_HUD.SetZoneContested` (`self.HUDWidgetRef`)))))

(event `HUD_UpdateZoneProgress`
  (params (NewProgress :type "Float (double-precision)"))
  (`/Engine/EditorBlueprintResources/StandardMacros.IsValid` (`self.HUDWidgetRef`)
    (:`Is Valid`
      (`/Game/Blueprints/WBP_HUD.UpdateZoneProgress` (`self.HUDWidgetRef`) NewProgress))))

(event `AddEnemyControl`
  (params (Amount :type "Float (double-precision)"))
  (if (and (`self.RoundActive`) (not (`self.MatchEnded`)))
    (set `self.EnemyControlPercent` (`KismetMathLibrary.FClamp` (+ (`self.EnemyControlPercent`) Amount) 0.0 100.0))
    (set `self.PlayerControlPercent` (`KismetMathLibrary.FClamp` (- (`self.PlayerControlPercent`) Amount) 0.0 100.0))
    (`/Engine/EditorBlueprintResources/StandardMacros.IsValid` (`self.HUDWidgetRef`)
      (:`Is Valid`
        (`self.HUD_UpdateTeamControl` (`self.PlayerControlPercent`) (`self.EnemyControlPercent`))
        (if (>= (`self.EnemyControlPercent`) 100.0)
          (`self.EndRoundDefeat`))))))

(event `HUD_SetZoneCaptured`
  (`/Engine/EditorBlueprintResources/StandardMacros.IsValid` (`self.HUDWidgetRef`)
    (:`Is Valid`
      (`/Game/Blueprints/WBP_HUD.SetZoneCaptured` (`self.HUDWidgetRef`)))))

(event `Telemetry_PrintSummary`
  (`KismetSystemLibrary.PrintString` "===== MATCH TEST SUMMARY =====")
  (`KismetSystemLibrary.PrintString` (`KismetTextLibrary.Conv_TextToString` (`|FormatText` "Duration: {Telemetry_MatchDuration}s" (`KismetMathLibrary.Round` (`self.Telemetry_MatchDuration`)))))
  (`KismetSystemLibrary.PrintString` (`KismetTextLibrary.Conv_TextToString` (`|FormatText` "Final Control: {PlayerControlPercent}%" (`KismetMathLibrary.Round` (`self.PlayerControlPercent`)))))
  (`KismetSystemLibrary.PrintString` (`KismetTextLibrary.Conv_TextToString` (`|FormatText` "Player Deaths: {Telemetry_PlayerDeaths}" (`self.Telemetry_PlayerDeaths`))))
  (`KismetSystemLibrary.PrintString` (`KismetTextLibrary.Conv_TextToString` (`|FormatText` "Bot Deaths: {Telemetry_BotDeaths}" (`self.Telemetry_BotDeaths`))))
  (`KismetSystemLibrary.PrintString` (`KismetTextLibrary.Conv_TextToString` (`|FormatText` "Time To First Kill: {Telemetry_TimeToFirstKill}s" (`self.Telemetry_TimeToFirstKill`))))
  (`KismetSystemLibrary.PrintString` (`KismetTextLibrary.Conv_TextToString` (`|FormatText` "Time To First Contest: {Telemetry_TimeToFirstZoneContest}s" (`self.Telemetry_TimeToFirstZoneContest`))))
  (`KismetSystemLibrary.PrintString` (`KismetTextLibrary.Conv_TextToString` (`|FormatText` "Immediate Restart: {Telemetry_ImmediateRestart}" (`self.Telemetry_ImmediateRestart`))))
  (`KismetSystemLibrary.PrintString` "Manual Note - Objective Understood: YES / NO")
  (`KismetSystemLibrary.PrintString` "Manual Note - Wanted Replay: YES / NO"))

(event `AddPlayerControl`
  (params (Amount :type "Float (double-precision)"))
  (if (and (`self.RoundActive`) (not (`self.MatchEnded`)))
    (set `self.PlayerControlPercent` (`KismetMathLibrary.FClamp` (+ (`self.PlayerControlPercent`) Amount) 0.0 100.0))
    (set `self.EnemyControlPercent` (`KismetMathLibrary.FClamp` (- (`self.EnemyControlPercent`) Amount) 0.0 100.0))
    (`/Engine/EditorBlueprintResources/StandardMacros.IsValid` (`self.HUDWidgetRef`)
      (:`Is Valid`
        (`self.HUD_UpdateTeamControl` (`self.PlayerControlPercent`) (`self.EnemyControlPercent`))
        (if (>= (`self.PlayerControlPercent`) 100.0)
          (`self.EndRoundVictory`))))))

(event `HUD_SetDefeat`
  (`/Engine/EditorBlueprintResources/StandardMacros.IsValid` (`self.HUDWidgetRef`)
    (:`Is Valid`
      (`/Game/Blueprints/WBP_HUD.SetDefeat` (`self.HUDWidgetRef`)))))

(event `HUD_SetDraw`
  (`/Engine/EditorBlueprintResources/StandardMacros.IsValid` (`self.HUDWidgetRef`)
    (:`Is Valid`
      (`/Game/Blueprints/WBP_HUD.SetDraw` (`self.HUDWidgetRef`)))))

(event `HUD_SetVictory`
  (`/Engine/EditorBlueprintResources/StandardMacros.IsValid` (`self.HUDWidgetRef`)
    (:`Is Valid`
      (`/Game/Blueprints/WBP_HUD.SetVictory` (`self.HUDWidgetRef`)))))

(event `Telemetry_RegisterRestartPressed`
  (if (`self.MatchEnded`)
    (if (<= (- (`KismetSystemLibrary.GetGameTimeInSeconds`) (`self.Telemetry_MatchEndTime`)) 3.0)
      (set `self.Telemetry_ImmediateRestart` true)
      (`KismetSystemLibrary.PrintString` "IMMEDIATE RESTART: TRUE"))))

(event `HUD_ShowRestartText`
  (`/Engine/EditorBlueprintResources/StandardMacros.IsValid` (`self.HUDWidgetRef`)
    (:`Is Valid`
      (`/Game/Blueprints/WBP_HUD.ShowRestartText` (`self.HUDWidgetRef`)))))

(event `Telemetry_RegisterPlayerDeath`
  (set `self.Telemetry_PlayerDeaths` (+ (`self.Telemetry_PlayerDeaths`) 1)))

(event `Telemetry_RegisterBotDeath`
  (set `self.Telemetry_BotDeaths` (+ (`self.Telemetry_BotDeaths`) 1))
  (if (< (`self.Telemetry_TimeToFirstKill`) 0.0)
    (set `self.Telemetry_TimeToFirstKill` (- (`KismetSystemLibrary.GetGameTimeInSeconds`) (`self.Telemetry_MatchStartTime`)))))

(event `UpdateRoundTimer`
  (params (DeltaSeconds :type "Float (double-precision)"))
  (set `self.RoundTime` (`KismetMathLibrary.FClamp` (- (`self.RoundTime`) DeltaSeconds) 0.0 (`self.RoundDuration`)))
  (set `self.TimerHUDAccumulator` (+ (`self.TimerHUDAccumulator`) DeltaSeconds))
  (if (>= (`self.TimerHUDAccumulator`) 0.1)
    (`self.HUD_UpdateTimer` (`self.RoundTime`))
    (set `self.TimerHUDAccumulator` 0.0)))

(event `HUD_ShowLowHealth`
  (`/Engine/EditorBlueprintResources/StandardMacros.IsValid` (`self.HUDWidgetRef`)
    (:`Is Valid`
      (`/Game/Blueprints/WBP_HUD.ShowLowHealth` (`self.HUDWidgetRef`)))))

(event `HUD_HideLowHealth`
  (`/Engine/EditorBlueprintResources/StandardMacros.IsValid` (`self.HUDWidgetRef`)
    (:`Is Valid`
      (`/Game/Blueprints/WBP_HUD.HideLowHealth` (`self.HUDWidgetRef`)))))

(event `HUD_UpdateTeamControl`
  (params (PlayerPercent :type "Float (double-precision)") (EnemyPercent :type "Float (double-precision)"))
  (`/Engine/EditorBlueprintResources/StandardMacros.IsValid` (`self.HUDWidgetRef`)
    (:`Is Valid`
      (`/Game/Blueprints/WBP_HUD.UpdateTeamControl` (`self.HUDWidgetRef`) PlayerPercent EnemyPercent))))

(event `FinalizeRound`
  (set `self.MatchEnded` true)
  (set `self.RoundActive` false)
  (set `self.Telemetry_MatchDuration` (- (`KismetSystemLibrary.GetGameTimeInSeconds`) (`self.Telemetry_MatchStartTime`)))
  (set `self.Telemetry_MatchEndTime` (`KismetSystemLibrary.GetGameTimeInSeconds`))
  (`self.Telemetry_PrintSummary`)
  (`self.HUD_ShowRestartText`))

(event `HUD_ShowDamageFlash`
  (`/Engine/EditorBlueprintResources/StandardMacros.IsValid` (`self.HUDWidgetRef`)
    (:`Is Valid`
      (`/Game/Blueprints/WBP_HUD.ShowDamageFlash` (`self.HUDWidgetRef`)))))

(event `HUD_UpdateHealth`
  (params (NewHealth :type "Float (double-precision)"))
  (`/Engine/EditorBlueprintResources/StandardMacros.IsValid` (`self.HUDWidgetRef`)
    (:`Is Valid`
      (`/Game/Blueprints/WBP_HUD.UpdateHealth` (`self.HUDWidgetRef`) NewHealth))))

(event `HUD_UpdateTimer`
  (params (TimeRemaining :type "Float (double-precision)"))
  (`/Engine/EditorBlueprintResources/StandardMacros.IsValid` (`self.HUDWidgetRef`)
    (:`Is Valid`
      (`/Game/Blueprints/WBP_HUD.UpdateTimer` (`self.HUDWidgetRef`) TimeRemaining))))

(event `HUD_ShowHitMarker`
  (`/Engine/EditorBlueprintResources/StandardMacros.IsValid` (`self.CrossHairWidgetRef`)
    (:`Is Valid`
      (`/Game/Blueprints/WBP_Crosshair.ShowHitMarker` (`self.CrossHairWidgetRef`)))))

(event `Telemetry_RegisterFirstZoneContest`
  (if (< (`self.Telemetry_TimeToFirstZoneContest`) 0.0)
    (set `self.Telemetry_TimeToFirstZoneContest` (- (`KismetSystemLibrary.GetGameTimeInSeconds`) (`self.Telemetry_MatchStartTime`)))))

(event `InitializeHUD`
  (bind _returnvalue (`|CreateWidget` "/Game/Blueprints/WBP_HUD.WBP_HUD_C" (`GameplayStatics.GetPlayerController` 0)))
  (bind _output_get (set `self.HUDWidgetRef` _returnvalue))
  (`UserWidget.AddToViewport` _output_get 0)
  (bind _returnvalue_2 (`|CreateWidget` "/Game/Blueprints/WBP_Crosshair.WBP_Crosshair_C" (`GameplayStatics.GetPlayerController` 0)))
  (bind _output_get_2 (set `self.CrossHairWidgetRef` _returnvalue_2))
  (`UserWidget.AddToViewport` _output_get_2 0)
  (`/Game/Blueprints/WBP_HUD.HideRestartText` (`self.HUDWidgetRef`))
  (`self.HUD_UpdateHealth` 100.0)
  (`self.HUD_UpdateTimer` (`self.RoundTime`))
  (`self.HUD_UpdateTeamControl` 0.0)
  (`self.HUD_UpdateCrowdEnergy` 0.0)
  (`self.HUD_SetZoneNeutral`))

(event `self.ReceiveBeginPlay`
  (set `self.RoundActive` true)
  (set `self.MatchEnded` false)
  (set `self.RoundTime` (`self.RoundDuration`))
  (set `self.PlayerControlPercent` 0.0)
  (set `self.EnemyControlPercent` 0.0)
  (set `self.CrowdEnergy` 0.0)
  (set `self.OverloadActive` false)
  (set `self.Telemetry_MatchStartTime` (`KismetSystemLibrary.GetGameTimeInSeconds`))
  (set `self.Telemetry_PlayerDeaths` 0)
  (set `self.Telemetry_BotDeaths` 0)
  (set `self.Telemetry_TimeToFirstKill` -1.0)
  (set `self.Telemetry_TimeToFirstZoneContest` -1.0)
  (set `self.Telemetry_ImmediateRestart` false)
  (`self.InitializeHUD`))

(event `CheckRoundEnd`
  (if (<= (`self.RoundTime`) 0.0)
    (`self.EndRoundByTimer`)))

(event `self.ReceiveTick`
  (params (DeltaSeconds :type "Float (single-precision)"))
  (if (and (`self.RoundActive`) (not (`self.MatchEnded`)))
    (`self.UpdateRoundTimer` DeltaSeconds)
    (`self.CheckRoundEnd`)))

(event `EndRoundByTimer`
  (if (> (`self.PlayerControlPercent`) (`self.EnemyControlPercent`))
    (`self.EndRoundVictory`)
    (elif (> (`self.EnemyControlPercent`) (`self.PlayerControlPercent`))
      (`self.EndRoundDefeat`)
      (else
        (`self.EndRoundDraw`)))))

(event `HUD_UpdateCrowdEnergy`
  (params (Energy :type "Float (double-precision)"))
  (`/Engine/EditorBlueprintResources/StandardMacros.IsValid` (`self.HUDWidgetRef`)
    (:`Is Valid`
      (`/Game/Blueprints/WBP_HUD.UpdateCrowdEnergy` (`self.HUDWidgetRef`) Energy))))

(event `EndRoundDefeat`
  (if (not (`self.MatchEnded`))
    (`self.HUD_SetDefeat`)
    (`self.FinalizeRound`)))

(event `EndRoundDraw`
  (if (not (`self.MatchEnded`))
    (`self.HUD_SetDraw`)
    (`self.FinalizeRound`)))

(event `EndRoundVictory`
  (if (not (`self.MatchEnded`))
    (`self.HUD_SetVictory`)
    (`self.FinalizeRound`)))

(event `HUD_SetOverloadState`
  (`/Engine/EditorBlueprintResources/StandardMacros.IsValid` (`self.HUDWidgetRef`)
    (:`Is Valid`
      (`/Game/Blueprints/WBP_HUD.SetOverloadState` (`self.HUDWidgetRef`)))))

(fn `UserConstructionScript`)